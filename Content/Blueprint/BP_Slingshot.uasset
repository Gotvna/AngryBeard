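; Slingshot actor that spawns a bird on BeginPlay and visually strings two ropes between its fork points and that bird.
; Every tick, StretchSlingRope updates the left and right rope meshes from mirrored local attach offsets transformed into world space.
; Each rope is placed at the midpoint to the bird, rotated along the connecting vector and scaled in X by distance, faking elastic bands without physics.
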(event `self.ReceiveBeginPlay`
  (`self.SpawnBird` (`self.Bird Class`)))

(event `self.ReceiveTick`
  (params (DeltaSeconds :type "Float (single-precision)"))
  (`self.Stretch Sling Rope` (`self.RopeRight`) (0.0 75.0 150.0))
  (`self.Stretch Sling Rope` (`self.RopeLeft`) (0.0 -75.0 150.0)))

(fn `Stretch Sling Rope`
  (params (`Rope Mesh` :type "StaticMeshComponent Object Reference") (`Attach Location` :type "Vector Structure"))
  (bind _returnvalue (`self.K2_GetActorLocation` (`self.Bird`)))
  (bind _returnvalue_2 (`KismetMathLibrary.TransformLocation` (`self.GetTransform`) `Attach Location`))
  (bind _returnvalue_3 (- _returnvalue_2 _returnvalue))
  (`SceneComponent.K2_SetWorldTransform` `Rope Mesh` (`KismetMathLibrary.MakeTransform` (* (+ _returnvalue_2 _returnvalue) 0.5) (`KismetMathLibrary.MakeRotFromX` _returnvalue_3) (`KismetMathLibrary.MakeVector` (* (`KismetMathLibrary.VSize` _returnvalue_3) 0.01) 0.05 0.05)) false false))

(fn `UserConstructionScript`)